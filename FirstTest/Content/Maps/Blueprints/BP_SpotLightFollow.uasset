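; Spotlight actor that turns to track the player while the player is inside its overlap area.
; Begin and end overlap events set a flag when the overlapping actor passes the IsPlayer check.
; While the flag is set, Tick calls LookAtPlayer, which smoothly interpolates the light's world rotation toward the first player pawn.
; The light keeps its last rotation once the player leaves.
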(event `self.ReceiveActorBeginOverlap`
  (params (OtherActor :type "Actor Object Reference"))
  (`/Game/Maps/Blueprints/Library/MacrosLibrary.IsPlayer` OtherActor
    (:`True`
      (set `self.IsPlayerOverlap` true))))

(event `self.ReceiveActorEndOverlap`
  (params (OtherActor :type "Actor Object Reference"))
  (`/Game/Maps/Blueprints/Library/MacrosLibrary.IsPlayer` OtherActor
    (:`True`
      (set `self.IsPlayerOverlap` false))))

(event `self.ReceiveTick`
  (params (DeltaSeconds :type "Float (single-precision)"))
  (if (`self.IsPlayerOverlap`)
    (`self.LookAtPlayer` DeltaSeconds)))

(fn `LookAtPlayer`
  (params (DeltaTime :type "Float (double-precision)"))
  (bind _spotlight (`self.SpotLight`))
  (`SceneComponent.K2_SetWorldRotation` (`self.SpotLight`) (`KismetMathLibrary.RInterpTo` (`SceneComponent.K2_GetComponentRotation` _spotlight) (`KismetMathLibrary.FindLookAtRotation` (`SceneComponent.K2_GetComponentLocation` _spotlight) (`self.K2_GetActorLocation` (`GameplayStatics.GetPlayerPawn` 0))) DeltaTime 2.0) false false))

(fn `UserConstructionScript`)