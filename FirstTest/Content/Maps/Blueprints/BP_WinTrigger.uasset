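; BP_WinTrigger is a level exit trigger that clears the level when the player enters it with every crystal collected.
; On BeginPlay it counts BP_Crystal actors and stores the total in the GameInstance.
; On player overlap it compares the collected count to that total, then either saves the BP_UI level timer to the GameInstance and prints a pass message, or prints that crystals are still missing.
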(event `self.ReceiveBeginPlay`
  (bind _outactors (`GameplayStatics.GetAllActorsOfClass` "/Game/Maps/Blueprints/BP_Crystal.BP_Crystal_C"))
  (set `/Game/Maps/Blueprints/BP_GameInstance.AllCrystalNum` (`KismetArrayLibrary.Array_Length` _outactors) (`/Game/Maps/Blueprints/Library/MacrosLibrary.GetGameInstance`)))

(event `self.ReceiveActorBeginOverlap`
  (params (OtherActor :type "Actor Object Reference"))
  (`/Game/Maps/Blueprints/Library/MacrosLibrary.IsPlayer` OtherActor
    (:`True`
      (if (`self.IsCollectAllCrystals`)
        (`self.SaveGameTime`)
        (`KismetSystemLibrary.PrintString` "过关!")
        (else
          (`KismetSystemLibrary.PrintString` "未收集完!"))))))

(fn `IsCollectAllCrystals`
  (returns (ReturnValue :type Boolean))
  (bind _bp_game_instance (`/Game/Maps/Blueprints/Library/MacrosLibrary.GetGameInstance`))
  (return (== (`/Game/Maps/Blueprints/BP_GameInstance.CollectCrystalNum` _bp_game_instance) (`/Game/Maps/Blueprints/BP_GameInstance.AllCrystalNum` _bp_game_instance))))

(fn `SaveGameTime`
  (bind _foundwidgets (`WidgetBlueprintLibrary.GetAllWidgetsOfClass` "/Game/Maps/Blueprints/BP_UI.BP_UI_C"))
  (set `/Game/Maps/Blueprints/BP_GameInstance.GameTime` (`/Game/Maps/Blueprints/BP_UI.LevelTime` (`|GetArrayItem` _foundwidgets)) (`/Game/Maps/Blueprints/Library/MacrosLibrary.GetGameInstance`)))

(fn `UserConstructionScript`)