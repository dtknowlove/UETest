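; BP_Cannon is a cannon actor that fires projectiles automatically and repeatedly from BeginPlay.
; After each FireRate delay, it activates the fire particle, plays a sound and spawns a scaled BP_Projectile at ProjectilePoint.
; A timeline animates the cannon mesh along its local Y axis, and its Fire Start event track loops back to the delay for the next shot.
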(event `self.ReceiveBeginPlay`
  (bind _fireparticle (`self.FireParticle`))
  (`KismetSystemLibrary.Delay` (`self.FireRate`) :!label _label)
  (`ActorComponent.Activate` _fireparticle true)
  (`GameplayStatics.PlaySoundAtLocation` "/Game/Audios/FireCue.FireCue" (`SceneComponent.K2_GetComponentLocation` _fireparticle) (struct) 1.0 1.0 0.0 null null null)
  (`self.SpawnProjectile`)
  (bind (_direction _firelocation) (`Timeline|FireTimeline` :!via `PlayFromStart`)
    (:`Update`
      (`SceneComponent.K2_SetRelativeLocation` (`self.Cannon`) (`KismetMathLibrary.MakeVector` 0.0 _firelocation) false false))
    (:`FireStart`
      (goto _label))))

(fn `SpawnProjectile`
  (bind _projectilepoint (`self.ProjectilePoint`))
  (`|SpawnActorFromClass` "/Game/Maps/Blueprints/BP_Projectile.BP_Projectile_C" (`KismetMathLibrary.MakeTransform` (`SceneComponent.K2_GetComponentLocation` _projectilepoint) (`SceneComponent.K2_GetComponentRotation` _projectilepoint) (`KismetMathLibrary.Conv_DoubleToVector` (`self.ProjectileScale`))) "Undefined" "OverrideRootScale" null null))

(fn `UserConstructionScript`)